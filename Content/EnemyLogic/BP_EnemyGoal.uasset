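; BP_EnemyGoal is a tower defence waypoint that forms the enemy path through a chain of NextGoal references.
; Overlapping enemies receive the next goal via an interface message, or at the final point damage the tower through GM_TowerDefence and are destroyed.
; Both cases play a sound when audio assistance is enabled.
; The construction script previews the path with cables, order labels, arrows and an end marker; BeginPlay reattaches the cable.
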(event OnComponentBeginOverlap(Sphere)
  (params (OverlappedComponent :type Primitive%20Component%20Object%20Reference) (OtherActor :type Actor%20Object%20Reference) (OtherComp :type Primitive%20Component%20Object%20Reference) (OtherBodyIndex :type Integer) (bFromSweep :type Boolean) (SweepResult :type Hit%20Result%20Structure%20%28by%20ref%29))
  ;[1 0 0.7969] Checks to make sure that the thing is an enemy
  (bind _asbp_master_enemy (Utilities|Casting|CastToBP_MasterEnemy OtherActor))
  ;[0 1 0.3672] Checks if this is the final Point or not
  (if (Variables|Default|GetFinalPoint)
    (Utilities|FlowControl|Sequence
      (:then_0
        ;[0.2422 0 1] play sound when enermy reaches the end
        (bind _asbp_gameinstance (Utilities|Casting|CastToBP_gameinstance (Game|GetGameInstance)))
        (if (Variables|/Game/UI/BP_gameinstance.BP_gameinstance_C|Getaudio%20assistance _asbp_gameinstance)
          (Utilities|FlowControl|Delay 0.01)
          (Audio|Components|Audio|Play (Variables|Default|GetAudio1) 0.0)))
      (:then_1
        ;[0.9688 0 1] Sends damage through to the game mode that hold the tower life total
        (bind _asgm_tower_defence (Utilities|Casting|CastToGM_TowerDefence (Game|GetGameMode)))
        (Default|EnemyReachedGoal _asgm_tower_defence (Variables|Default|GetDamage))
        ;[1 0.6094 0] Deletes the enemy from the game instance
        (Actor|DestroyActor _asbp_master_enemy)))
    (else
      (Utilities|FlowControl|Sequence
        (:then_0
          ;[0.2422 0 1] play sound when enermy reaches the end
          (bind _asbp_gameinstance_2 (Utilities|Casting|CastToBP_gameinstance (Game|GetGameInstance)))
          (if (Variables|/Game/UI/BP_gameinstance.BP_gameinstance_C|Getaudio%20assistance _asbp_gameinstance_2)
            (Utilities|FlowControl|Delay 0.01)
            (Audio|Components|Audio|Play (Variables|Default|GetAudio) 0.0)))
        (:then_1
          ;[0 0.5781 1] Lets the enemy know where to go through sending a message through the Enemy interface
          (Class|BPEnemyInterface|GetInstructions(Message) _asbp_master_enemy (Variables|Default|GetNext%20Goal)))))))

(event EventBeginPlay
  (bind _next_goal (Variables|Default|GetNext%20Goal))
  ;[0 1 0.1328] Fixes issue where cable path gets detached on play
  (Utilities|IsValid _next_goal
    (:Is%20Valid
      (Class|CableComponent|SetAttachEndtoComponent (Variables|Default|GetCable) (Variables|BP_EnemyGoal_C|GetCable _next_goal) "None"))))

(fn ConstructionScript
  (bind _pointorder (Variables|Default|GetPointOrder))
  (bind _cone (Variables|Default|GetCone))
  (bind _cone_2 (Variables|Default|GetCone))
  ;[1 1 1] Attaches cable to next goal to show path
  (Class|CableComponent|SetAttachEndtoComponent (Variables|Default|GetCable) (Variables|BP_EnemyGoal_C|GetCone (Variables|Default|GetNext%20Goal)) "None")
  ;[1 1 1] Sets the colour and label of text for goals
  (Rendering|Components|TextRender|SetText _pointorder (Utilities|Text|ToText(Integer) (Variables|Default|GetPointSequence)))
  (Rendering|Components|TextRender|SetTextRenderColor _pointorder (Variables|Default|GetValue))
  (if (Variables|Default|GetFinalPoint)
    ;[1 1 1] Sets mesh based on being the end goal
    (Components|StaticMesh|SetStaticMesh _cone_2 "/Engine/BasicShapes/Cylinder.Cylinder")
    (Transformation|SetRelativeScale3D _cone_2 "3.000000,3.000000,0.100000")
    (Transformation|AddLocalOffset _cone_2 "0, 0,-100.000000" false false)
    (else
      ;[1 1 1] Sets and rotates arrown mesh to face the next goal
      (Components|StaticMesh|SetStaticMesh _cone "/Engine/VREditor/LaserPointer/CursorPointer.CursorPointer")
      (Transformation|SetRelativeScale3D _cone "1.000000,0.250000,0.250000")
      (Transformation|SetWorldRotation _cone (Math|Rotator|FindLookatRotation (Transformation|GetActorLocation self) (Transformation|GetActorLocation (Variables|Default|GetNext%20Goal))) false false))))