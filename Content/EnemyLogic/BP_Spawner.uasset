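; Enemy spawner that shows a ghost preview of an enemy type and a cable marking the path to its goal.
; The game mode calls Activate to spawn the chosen class at the arrow, pass it EnemyGoal via interface message, and preview the next enemy.
; Construction attaches the cable and builds the ghost mesh from Wave1's last data-table entry.
; BeginPlay reattaches the cable and starts a looping "Round Start" timer, whose function is not defined here.
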(event Custom|Activate
  (params (TypeOfEnemy :type Integer) (Next%20Up :type Integer))
  ;[0.3125 0 1] This is a custom event we call from the GM
  (CallFunction|UpdatePreviewMesh Next%20Up)
  (bind _returnvalue (Game|SpawnActorfromClass (Utilities|Array|Get(acopy) (Variables|Default|GetClass) TypeOfEnemy) (Math|Transform|MakeTransform (Transformation|GetWorldLocation (Variables|Default|GetArrow)) "0, 0, 0" "1.000000,1.000000,1.000000") "AdjustIfPossibleButAlwaysSpawn" "SelectDefaultAtRuntime" 0 0))
  ;[0 1 0.6953] IS Valid just checks that it actually did spawn, so it can do the next thing without throwing a fit
  (Utilities|IsValid _returnvalue
    (:Is%20Valid
      ;[0.05469 1 0] This sends a message to our BP Interface for something (the enemy) to recieve.
      (Class|BPEnemyInterface|GetInstructions(Message) _returnvalue (Variables|Default|GetEnemy%20Goal)))))

(event EventBeginPlay
  ;[0.4297 0 1] When the game starts, this timer starts and loops
  (Utilities|Time|SetTimerbyFunctionName 0 "Round Start" (Variables|Default|GetSpawnRate) true)
  ;[0.7344 1 0] Fixes issue where cable path gets detached on play
  (Class|CableComponent|SetAttachEndtoComponent (Variables|Default|GetCable) (Variables|/Game/EnemyLogic/BP_EnemyGoal.BP_EnemyGoal_C|GetCable (Variables|Default|GetEnemy%20Goal)) "None"))

(event EventTick
  (params (DeltaSeconds :type Float%20%28single-precision%29)))

(fn ConstructionScript
  (bind _skeletalmesh (Variables|Default|GetSkeletalMesh))
  ;[1 1 1] Attaches cable to next goal to show path
  (Class|CableComponent|SetAttachEndtoComponent (Variables|Default|GetCable) (Variables|/Game/EnemyLogic/BP_EnemyGoal.BP_EnemyGoal_C|GetCone (Variables|Default|GetEnemy%20Goal)) "None")
  (bind _returnvalue (Utilities|GetDataTableRow "/Game/GameRules/WaveData.WaveData" "Wave1")
    (:then
      (Components|SkinnedMesh|SetSkinnedAssetandUpdate _skeletalmesh (Utilities|Array|Get(acopy) (Variables|Default|GetEnemyMeshes) (Utilities|Array|Get(acopy) (.enemytospawn _returnvalue) (- (Utilities|Array|Length (.enemytospawn _returnvalue)) 1))) true)
      ;[1 1 1] loops through all materials the mesh may have and sets them to the ghost material
      (for (_ _array_index) (Class|MeshComponent|GetMaterialSlotNames _skeletalmesh)
        (Rendering|Material|SetMaterial _skeletalmesh _array_index "/Game/ARTassets/GhostMaterial_Inst.GhostMaterial_Inst")))))

(fn UpdatePreviewMesh
  (params (NextUP :type Integer))
  (Components|SkinnedMesh|SetSkinnedAssetandUpdate (Variables|Default|GetSkeletalMesh) (Utilities|Array|Get(acopy) (Variables|Default|GetEnemyMeshes) NextUP) true))