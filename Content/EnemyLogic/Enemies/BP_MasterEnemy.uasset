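; BP_MasterEnemy is the tower defence enemy that walks to a goal and dies to projectile damage.
; GetInstructions receives a goal and starts an AI MoveTo toward it, while capsule overlaps with BP_MasterProjectile subtract that projectile's damage from health.
; At zero health it awards money through GM_TowerDefence, spawns an explosion and notifies every tower to drop it as a target.
; DestroyActor sits inside that tower loop, and StatusEffect is an empty stub.
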(event OnComponentBeginOverlap(CapsuleComponent)
  (params (OverlappedComponent :type Primitive%20Component%20Object%20Reference) (OtherActor :type Actor%20Object%20Reference) (OtherComp :type Primitive%20Component%20Object%20Reference) (OtherBodyIndex :type Integer) (bFromSweep :type Boolean) (SweepResult :type Hit%20Result%20Structure%20%28by%20ref%29))
  ;[1 1 1] Checks if the thing that hit is is a projectile
  (bind _asbp_master_projectile (Utilities|Casting|CastToBP_MasterProjectile OtherActor))
  ;[1 1 1] Reduces health and compare the new value to ZERO
  (bind _output_get (Variables|Default|SetEnemyHealth (- (Variables|Default|GetEnemyHealth) (Variables|/Game/Character_Towers/BP_MasterProjectile.BP_MasterProjectile_C|GetDamage _asbp_master_projectile))))
  (if (<= _output_get 0)
    (bind _asgm_tower_defence (Utilities|Casting|CastToGM_TowerDefence (Game|GetGameMode)))
    (Default|AddMoney _asgm_tower_defence (Variables|Default|GetValue))
    ;[1 1 1] Spawns Explosion when life at ZERO
    (Effects|SpawnEmitteratLocation "/Game/StarterContent/Particles/P_Explosion.P_Explosion" (Transformation|GetActorLocation self))
    ;[1 1 1] Tells all towers that this is no longer a valid target and to remove it from thier list
    (bind _outactors (Actor|GetAllActorsOfClass "/Game/Character_Towers/BP_MasterBasicTower.BP_MasterBasicTower_C"))
    (for _array_element _outactors
      (Default|TargetDied _array_element self)
      ;[1 1 1] Deletes the enemy from existence
      (Actor|DestroyActor))))

(event Custom|Status%20Effect)

(event EventGetInstructions
  (params (Goal :type BP%20Enemy%20Goal%20Object%20Reference))
  ;[1 1 1] This si the Goal message being recieved from goals or spawners
  ;[1 1 1] This is the "AI" of our enemies
  (AI|AIMoveTo self "0, 0, 0" Goal 5.0 false))

(fn ConstructionScript)