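; Tower defence game mode that runs waves, money, tower lives and win or lose states.
; Each planning phase loads the next wave's enemy list from the WaveData table and waits for EndPlanningPhase.
; A looping one-second timer then feeds enemies, last entry first, to a spawner with next-up previews.
; Clearing all waves plays a slow-motion post-process finish, while losing all tower health slows time.
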(event Custom|EnemyReachedGoal
  (params (Damage :type Integer))
  ;[1 0.5859 0] Deducting Tower Health
  (bind _output_get (Variables|Default|SetTowerLifePoints (Math|Integer|Clamp(Integer) (- (Variables|Default|GetTowerLifePoints) Damage) 0 10)))
  (if (<= _output_get 0)
    (Development|PrintString "Game Over")
    (Utilities|Time|SetGlobalTimeDilation 0.1)
    (else
      (Development|PrintString (Utilities|String|Append (Utilities|String|ToString(Integer) _output_get) " Tower Health Left"))
      (Audio|PlaySound2D "/Engine/VREditor/Sounds/UI/Camera_Shutter.Camera_Shutter" 1.0 1.0 0.0 0 0))))

(event Custom|SpawnerActivate
  (bind _enemylist (Variables|Default|GetEnemyList))
  (bind _enemyspawnpoints (Variables|Default|GetEnemySpawnpoints))
  (bind _spawnertoactivate (Variables|Default|GetSpawnerToActivate))
  (bind _output (Utilities|Array|Get(acopy) _enemyspawnpoints _spawnertoactivate))
  ;[0 0.3906 1] Checks if wave is valid
  (bind _outactors (Actor|GetAllActorsOfClass "/Game/EnemyLogic/Enemies/BP_MasterEnemy.BP_MasterEnemy_C"))
  (if (and (> (Variables|Default|GetWaveNumber) (Variables|Default|GetWaveTotal)) (== (Utilities|Array|Length _outactors) 0))
    ;[0.4062 0 1] Level End Logic
    (Development|PrintString "LEVEL COMPLETE")
    (bind _outactors_2 (Actor|GetAllActorsOfClass "/Script/Engine.PostProcessVolume"))
    (bind (_direction _floattrack _newtrack_1) (Timeline|Timeline_0 Play)
      (:Update
        (Utilities|Time|SetGlobalTimeDilation (Math|Float|Lerp 1.0 0.25 _floattrack))
        (Variables|/Script/Engine.PostProcessVolume|SetSettings (Utilities|Array|Get(acopy) _outactors_2) (Utilities|Struct|MakePostProcessSettings (Math|Vector4|MakeVector4 (Math|Float|Lerp 1.2 0.5 _newtrack_1) (Math|Float|Lerp 1.2 0.5 _newtrack_1) (Math|Float|Lerp 1.2 0.5 _newtrack_1) 1.0)))))
    (else
      ;[0.5703 0 1] Will wait for player to start wave
      (if (not (Variables|Default|GetPlanningPhase))
        (if (> (Variables|Default|GetNumber%20Of%20Enemies%20in%20Wave) 0)
          (Default|Activate _output (Utilities|Array|Get(acopy) (Variables|Default|GetEnemyList) (- (Variables|Default|GetNumber%20Of%20Enemies%20in%20Wave) 1)) (Utilities|Array|Get(acopy) _enemylist (Math|Integer|Clamp(Integer) (- (Variables|Default|GetNumber%20Of%20Enemies%20in%20Wave) 2) 0 (Utilities|Array|Length _enemylist))))
          (Math|Integer|DecrementInt (Variables|Default|GetNumber%20Of%20Enemies%20in%20Wave))
          (else
            (CallFunction|RoundComplete)
            (for _array_element (Variables|Default|GetEnemySpawnpoints)
              (Default|UpdatePreviewMesh _array_element (Variables|Default|GetNext%20Up%28EmptyMeshValue%29)))))
        (else
          (Development|PrintString "Planning")
          (Default|UpdatePreviewMesh _output (Variables|Default|GetNext%20Up)))))))

(event Custom|Round%20Complete
  (bind _wavenumber (Variables|Default|GetWaveNumber))
  ;[1 0 0.9609] Progress Wave and retrieves new wave layout from Data table
  (bind _outactors (Actor|GetAllActorsOfClass "/Game/EnemyLogic/Enemies/BP_MasterEnemy.BP_MasterEnemy_C"))
  (if (== (Utilities|Array|Length _outactors) 0)
    (Variables|Default|SetPlanningPhase true)
    (Math|Integer|IncrementInt _wavenumber
      (:%20%20
        (bind _outrownames (DataTable|GetDataTableRowNames "/Game/GameRules/WaveData.WaveData"))
        (bind _output_get (Variables|Default|SetOut%20Row%20Names _outrownames))
        (bind _returnvalue (Utilities|GetDataTableRow "/Game/GameRules/WaveData.WaveData" (Utilities|Array|Get(acopy) _output_get (- _wavenumber 1)))
          (:then
            (bind _output_get_2 (Variables|Default|SetEnemyList (.enemytospawn _returnvalue)))
            (Variables|Default|SetNumber%20Of%20Enemies%20in%20Wave (Utilities|Array|Length _output_get_2))))))))

(event Custom|Init
  (bind _asbp_tower_defence_character (Utilities|Casting|CastToBP_TowerDefenceCharacter (Game|GetPlayerCharacter 0)))
  (Variables|Default|SetAs%20BP%20Tower%20Defence%20Character _asbp_tower_defence_character)
  (Utilities|Time|SetTimerbyEvent (delegate Custom|SpawnerActivate) 1.0 true 1.0))

(event Custom|EndPlanningPhase
  ;[1 0.3281 0] Ending Planning Phase
  (Variables|Default|SetPlanningPhase false))

(event Custom|SubtractMoney
  (params (Money%20Delta :type Integer))
  ;[0 1 0.4844] Update Money
  (Variables|Default|SetMoney (- (Variables|Default|GetMoney) Money%20Delta)))

(event Custom|AddMoney
  (params (MoneyDelta :type Integer))
  (bind _as_bp_tower_defence_character (Variables|Default|GetAs%20BP%20Tower%20Defence%20Character))
  ;[0 1 0.4844] Update Money
  (Variables|Default|SetMoney (+ (Variables|Default|GetMoney) MoneyDelta))
  (if (Variables|/Game/Characters/ThirdPerson/Blueprints/BP_TowerDefenceCharacter.BP_TowerDefenceCharacter_C|GetImBuilding _as_bp_tower_defence_character)
    (Default|UpdateBuildItem _as_bp_tower_defence_character)))

(event EventBeginPlay
  ;[1 0.6328 0] Game Start Logic
  (bind _returnvalue (UserInterface|CreateWidget "/Game/UI/UI_MainMenu.UI_MainMenu_C"))
  (UserInterface|Viewport|AddtoPlayerScreen _returnvalue 1)
  (bind _returnvalue_2 (UserInterface|CreateWidget "/Game/UI/HUD_PlayerChar.HUD_PlayerChar_C"))
  (UserInterface|Viewport|AddtoPlayerScreen _returnvalue_2)
  (bind _outrownames (DataTable|GetDataTableRowNames "/Game/GameRules/WaveData.WaveData"))
  (Variables|Default|SetWaveTotal (Utilities|Array|Length _outrownames))
  ;[1 0 0.9375] Creates list of all spawners in level
  (bind _outactors (Actor|GetAllActorsOfClass "/Game/EnemyLogic/BP_Spawner.BP_Spawner_C"))
  (Variables|Default|SetEnemySpawnpoints _outactors)
  (CallFunction|RoundComplete)
  (CallFunction|Init))

(fn ConstructionScript)