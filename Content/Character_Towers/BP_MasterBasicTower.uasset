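; Base tower for a tower defense game that starts as a non-colliding ghost, then activates if paid for or destroys itself.
; A LineOfSight sphere maintains a list of BP_MasterEnemy targets in range, also pruned when a target dies.
; Looping timers rotate an Arrow toward the first target and fire projectiles from it, with a Niagara effect given the target's position and bullet colour.
; Upgrade logic is an empty placeholder.
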(event OnComponentBeginOverlap(LineOfSight)
  (params (OverlappedComponent :type Primitive%20Component%20Object%20Reference) (OtherActor :type Actor%20Object%20Reference) (OtherComp :type Primitive%20Component%20Object%20Reference) (OtherBodyIndex :type Integer) (bFromSweep :type Boolean) (SweepResult :type Hit%20Result%20Structure%20%28by%20ref%29))
  ;[1 1 1] Add anything that eneters line of sight to potential target list
  (bind _asbp_master_enemy (Utilities|Casting|CastToBP_MasterEnemy OtherActor))
  (Utilities|Array|Add (Variables|Default|GetActiveTargets) _asbp_master_enemy))

(event OnComponentEndOverlap(LineOfSight)
  (params (OverlappedComponent :type Primitive%20Component%20Object%20Reference) (OtherActor :type Actor%20Object%20Reference) (OtherComp :type Primitive%20Component%20Object%20Reference) (OtherBodyIndex :type Integer))
  (bind _activetargets (Variables|Default|GetActiveTargets))
  ;[1 1 1] Removes targets from list if they leave line of sight
  (for (_ _array_index) _activetargets
    (if (== (Utilities|Array|Get(acopy) _activetargets _array_index) OtherActor)
      (Utilities|Array|RemoveIndex _activetargets _array_index))))

(event Custom|AimAtTarget
  (bind _arrow (Variables|Default|GetArrow))
  (bind _activetargets (Variables|Default|GetActiveTargets))
  (bind _output (Utilities|Array|Get(acopy) _activetargets))
  ;[1 1 1] Checks to see if we have any valid targets
  (Utilities|IsValid _output
    (:Is%20Valid
      ;[1 1 1] Enables/Disables firing logic
      (Variables|Default|SetIHaveSomethingToShootAt true)
      ;[1 1 1] Updates Aim Direction represented by Arrow
      (Transformation|SetWorldRotation (Variables|Default|GetArrow) (Math|Interpolation|RInterpTo (Transformation|GetWorldRotation _arrow) (Math|Rotator|FindLookatRotation (Transformation|GetWorldLocation _arrow) (Transformation|GetActorLocation _output)) 0.01 (Variables|Default|GetInterp%20Speed)) false false))
    (:Is%20Not%20Valid
      (Variables|Default|SetIHaveSomethingToShootAt false))))

(event Custom|TowerPlaced
  (bind _staticmesh (Variables|Default|GetStaticMesh))
  (Rendering|Material|SetMaterial _staticmesh 0 (Variables|Default|GetBuiltMaterial))
  (Collision|SetCollisionEnabled _staticmesh "QueryAndPhysics"))

(event Custom|ShootAtEnemy
  (bind _activetargets (Variables|Default|GetActiveTargets))
  (bind _arrow (Variables|Default|GetArrow))
  (bind _output (Utilities|Array|Get(acopy) _activetargets))
  ;[1 1 1] Checks to see if target is valid before actually shooting
  (if (Variables|Default|GetIHaveSomethingToShootAt)
    ;[1 1 1] Spawns the Projectile
    (Game|SpawnActorfromClass (Utilities|Array|Get(acopy) (Variables|Default|GetClass) (Variables|Default|GetAmmoType)) (Math|Transform|MakeTransform (Transformation|GetWorldLocation _arrow) (Transformation|GetWorldRotation _arrow) "1.000000,1.000000,1.000000") "Undefined" 0 0)
    ;[1 1 1] Niagara at Enemy
    (bind _returnvalue (Niagara|SpawnSystemAttached (Variables|Default|GetNiagaraSystemtoUse) (Variables|Default|GetArrow) "None" "0, 0, 0" "0, 0, 0" "KeepRelativeOffset" true))
    (Utilities|IsValid _returnvalue
      (:Is%20Valid
        (Utilities|IsValid _output
          (:Is%20Valid
            (Class|NiagaraComponent|SetVariablePosition _returnvalue "Thisone" (Transformation|GetActorLocation _output))
            (Niagara|SetNiagaraVariable(LinearColor) _returnvalue "TowerColour" (Variables|Default|GetBulletColour))))))))

(event Custom|Activate%20Tower
  (params (CostPaid? :type Boolean))
  (bind _staticmesh (Variables|Default|GetStaticMesh))
  ;[1 1 1] When Placed checks if paid for, if not destroys self, if so powers on
  (if CostPaid?
    (Rendering|Material|SetMaterial _staticmesh 0 (Variables|Default|GetBuiltMaterial))
    (Collision|SetCollisionEnabled _staticmesh "QueryAndPhysics")
    (Utilities|Time|SetTimerbyFunctionName 0 "AimAtTarget" 0.01 true)
    (Utilities|Time|SetTimerbyFunctionName 0 "ShootAtEnemy" (Variables|Default|GetFireRate) true)
    (else
      (Actor|DestroyActor))))

(event Custom|TargetDied
  (params (Target :type BP%20Master%20Enemy%20Object%20Reference))
  (bind _activetargets (Variables|Default|GetActiveTargets))
  ;[1 1 1] Cleans up any targets that are not longer valid so new target can be chosen
  (for (_array_element _array_index) _activetargets
    (if (== Target _array_element)
      (Utilities|Array|RemoveIndex _activetargets _array_index))))

(event Custom|UpgradeMytower
  ;[1 1 1] Space for upgrade logic
)

(event EventBeginPlay
  (bind _staticmesh (Variables|Default|GetStaticMesh))
  ;[1 1 1] Set Material
  (Variables|Default|SetBuiltMaterial (Rendering|Material|GetMaterial _staticmesh 0))
  (Rendering|Material|SetMaterial _staticmesh 0 "/Game/ARTassets/GhostMaterial_Inst1.GhostMaterial_Inst1")
  (Collision|SetCollisionEnabled _staticmesh "NoCollision"))

(fn ConstructionScript
  (Components|Sphere|SetSphereRadius (Variables|Default|GetLineOfSight) (Variables|Default|GetSphereofSightRadius) true))